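; Melee enemy AI that wanders to random navmesh points and chases pawns it sees at higher speed, resuming its slow wander after a retriggerable delay.
; When the player is close, a sighting plays an attack montage whose notify applies damage through a sphere overlap.
; Damage triggers hit reactions or death, which clears target lock, ragdolls, awards XP and later removes the mesh.
; Tick updates the health bar and turns it toward the camera.
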(event OnSeePawn(PawnSensing)
  (params (Pawn :type Pawn%20Object%20Reference))
  ;[1 1 1] Move to Player
  (bind _returnvalue (CallFunction|IsPlayerNear? false))
  (if _returnvalue
    (Utilities|FlowControl|DoOnce false :!label _label
      (:Completed
        (Animation|Montage|PlayMontage (Variables|Character|GetMesh) "/Game/BattleWizardPolyart/Animations/Anim_Montages/LightAttack_Montage.LightAttack_Montage"
          (:then
            (Utilities|FlowControl|Sequence :!label _label_2
              (:then_0
                (Utilities|FlowControl|DoOnce false
                  (:Completed
                    (Variables|/Script/Engine.CharacterMovementComponent|SetMaxWalkSpeed (Variables|Character|GetCharacterMovement) 2.5e+02))))
              (:then_1
                (AI|AIMoveTo self "0, 0, 0" Pawn 5.0 false
                  (:then
                    (Utilities|FlowControl|RetriggerableDelay 2.0)
                    (Variables|/Script/Engine.CharacterMovementComponent|SetMaxWalkSpeed (Variables|Character|GetCharacterMovement) 7e+01)
                    (CallFunction|CanSprintAgain)
                    (CallFunction|MovetoRandomLocation))))))
          (:OnCompleted
            (goto _label Reset))
          (:OnNotifyBegin
            (bind _outactors (Collision|SphereOverlapActors (Transformation|GetWorldLocation (Variables|Default|GetSphere)) 5e+01 (Utilities|Array|MakeArray "ObjectTypeQuery3") "/Game/ThirdPerson/Blueprints/BP_ThirdPersonCharacter.BP_ThirdPersonCharacter_C" (Utilities|Array|MakeArray self)))
            (for _array_element _outactors
              (Game|Damage|ApplyDamage _array_element 15.0 (Pawn|GetController) self "/Script/Engine.DamageType"))))))
    (else
      (goto _label_2))))

(event Custom|DummyDeath
  (bind _mesh (Variables|Character|GetMesh))
  ;[1 1 1] Dummy Death
  (bind _asbp_third_person_character (Utilities|Casting|CastToBP_ThirdPersonCharacter (Game|GetPlayerCharacter 0)))
  (Variables|/Game/ThirdPerson/Blueprints/BP_ThirdPersonCharacter.BP_ThirdPersonCharacter_C|SetIsValidTarget? _asbp_third_person_character false)
  (Variables|/Game/ThirdPerson/Blueprints/BP_ThirdPersonCharacter.BP_ThirdPersonCharacter_C|SetTargetLock? _asbp_third_person_character false)
  (Physics|SetSimulatePhysics _mesh true)
  (Audio|PlaySoundatLocation "/Game/Sounds/AttackCue.AttackCue" (Transformation|GetWorldLocation _mesh) "0, 0, 0" 1.0 1.0 0.0 0 0 0 0)
  (bind _asbp_third_person_character_2 (Utilities|Casting|CastToBP_ThirdPersonCharacter (Game|GetPlayerCharacter 0)))
  (Variables|/Game/ThirdPerson/Blueprints/BP_ThirdPersonCharacter.BP_ThirdPersonCharacter_C|SetXP _asbp_third_person_character_2 (+ (Variables|/Game/ThirdPerson/Blueprints/BP_ThirdPersonCharacter.BP_ThirdPersonCharacter_C|GetXP _asbp_third_person_character_2) 35.0))
  (Components|DestroyComponent (Variables|Collision|GetCapsuleComponent))
  (Rendering|SetVisibility (Variables|Default|GetHealth%20Bar%20Widget) false false)
  (Utilities|FlowControl|Delay 5.0)
  (Components|DestroyComponent (Variables|Character|GetMesh)))

(event Custom|TargetDummyFunc
  (bind _health_bar_widget (Variables|Default|GetHealth%20Bar%20Widget))
  ;[1 1 1] Target Dummy Func
  (bind _aswb_target_dummy_bar (Utilities|Casting|CastToWB_TargetDummyBar (UserInterface|GetWidget (Variables|Default|GetHealth%20Bar%20Widget))))
  (Progress|SetPercent (Variables|/Game/ProjectFiles/WB_TargetDummyBar.WB_TargetDummyBar_C|GetHealthBarDummy _aswb_target_dummy_bar) (/ (Variables|Default|GetHealth) (Variables|Default|GetMaxHealth)))
  (Transformation|SetWorldRotation _health_bar_widget (Math|Rotator|FindLookatRotation (Transformation|GetWorldLocation _health_bar_widget) (Transformation|GetWorldLocation (Variables|/Script/Engine.PlayerCameraManager|GetTransformComponent (Game|GetPlayerCameraManager 0)))) false false))

(event Custom|MoveToRandomLocation
  ;[1 1 1] movetorandomlocatin
  (bind _randomlocation (Class|NavigationSystemV1|GetRandomLocationinNavigableRadius (Transformation|GetActorLocation) 1e+03 0 0))
  (AI|AIMoveTo self _randomlocation 0 5.0 false
    (:OnSuccess
      (CallFunction|MovetoRandomLocation))))

(event Custom|CanSprintAgain
  ;[1 1 1] Move to Player
  (Utilities|FlowControl|DoOnce false) ; enters at Reset
)

(event EventBeginPlay
  (CallFunction|MovetoRandomLocation))

(event EventTick
  (params (DeltaSeconds :type Float%20%28single-precision%29))
  (CallFunction|TargetDummyFunc))

(event Game|Damage|EventAnyDamage
  (params (Damage :type Float%20%28single-precision%29) (DamageType :type Damage%20Type%20Object%20Reference) (InstigatedBy :type Controller%20Object%20Reference) (DamageCauser :type Actor%20Object%20Reference))
  ;[1 1 1] Take Damage
  (Utilities|FlowControl|DoOnce false :!label _label
    (:Completed
      (Utilities|Casting|CastToBP_ThirdPersonCharacter (Game|GetPlayerCharacter 0))
      (bind _output_get (Variables|Default|SetHealth (- (Variables|Default|GetHealth) Damage)))
      (if (<= _output_get 0.0)
        (CallFunction|DummyDeath)
        (else
          (Animation|PlayAnimMontage "/Game/BattleWizardPolyart/Animations/Anim_Montages/GetHitAnim_Montage.GetHitAnim_Montage" 1.0 "None")
          (Audio|PlaySoundatLocation "/Game/Sounds/AttackCue.AttackCue" (Transformation|GetWorldLocation (Variables|Character|GetMesh)) "0, 0, 0" 1.0 1.0 0.0 0 0 0 0)
          (goto _label Reset))))))

(fn ConstructionScript)

(fn IsPlayerNear?
  (params (Condition :type Boolean))
  (bind _asbp_third_person_character (Utilities|Casting|CastToBP_ThirdPersonCharacter (Game|GetPlayerCharacter 0)))
  (return (< (Transformation|GetHorizontalDistanceTo _asbp_third_person_character) 1e+02)))